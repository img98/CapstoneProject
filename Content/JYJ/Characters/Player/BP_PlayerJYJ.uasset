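; BP_PlayerJYJ is a player Blueprint that adds a test throw for distraction objects.
; Pressing the TestThrow input spawns a BP_DistractionObject slightly in front of and above the capsule.
; It then sets the object's sphere physics velocity along the line from the player to the spawn point, so that offset gives a fixed-speed, upward-angled lob.
; No other event or construction logic is active beyond the parent construction call.
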(event `self.ReceiveTick`
  (params (DeltaSeconds :type "Float (single-precision)")))

(event `InputAction|TestThrow`
  (params (Key :type "Key Structure"))
  (bind _capsulecomponent (`self.CapsuleComponent`))
  (:`Pressed`
    (bind _returnvalue (`|SpawnActorFromClass` "/Game/JYJ/414/BP_DistractionObject.BP_DistractionObject_C" (`KismetMathLibrary.MakeTransform` (+ (`SceneComponent.K2_GetComponentLocation` _capsulecomponent) (* (`SceneComponent.GetForwardVector` _capsulecomponent) 50.0) (0.0 0.0 50.0)) (`self.K2_GetActorRotation`)) "Undefined" "OverrideRootScale" null null))
    (`PrimitiveComponent.SetPhysicsLinearVelocity` (`/Game/JYJ/414/BP_DistractionObject.SphereCollision` _returnvalue) (* (`KismetMathLibrary.GetDirectionUnitVector` (`self.K2_GetActorLocation`) (`self.K2_GetActorLocation` _returnvalue)) 1000.0) false "None")))

(fn `UserConstructionScript`
  (`parent.UserConstructionScript`))